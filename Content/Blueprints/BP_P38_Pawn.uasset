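; BP_P38_Pawn is a player-controllable P-38 plane that flies forward continuously along its local X axis.
; Tick spins both propellers around roll, the right via RotatePropeller and the left with the same logic inline, and offsets the actor by MoveSpeed.
; Pitch and Roll axis inputs are clamped and scaled by RotationSpeed and delta time, but both currently rotate the actor in pitch.
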(event EventBeginPlay)

(event Collision|EventActorBeginOverlap
  (params (OtherActor :type Actor%20Object%20Reference)))

(event EventTick
  (params (DeltaSeconds :type Float%20%28single-precision%29))
  ;[1 1 1] Rotate Right
  (CallFunction|RotatePropeller (Variables|Default|GetRightPropeller))
  ;[1 1 1] Rotate Left
  (Transformation|AddLocalRotation (Variables|Default|GetLeftPropeller) (Math|Rotator|MakeRotator (* (Utilities|Time|GetWorldDeltaSeconds) (Variables|속력|GetPropellerRotationSpeed)) 0.0 0.0) false false)
  ;[1 1 1] Move Plane
  (Transformation|AddActorLocalOffset (Math|Vector|MakeVector (* (Utilities|Time|GetWorldDeltaSeconds) (Variables|속력|GetMoveSpeed)) 0.0 0.0) false false))

(event Input|ActionEvents|InputActionFire
  (params (Key :type Key%20Structure :default "None")))

(event Input|AxisEvents|InputAxisPitch
  (params (AxisValue :type Float%20%28single-precision%29))
  (Transformation|AddActorLocalRotation (Math|Rotator|MakeRotator 0.0 (* (Math|Float|Clamp(Float) AxisValue -1.0) (Utilities|Time|GetWorldDeltaSeconds) (Variables|Default|GetRotationSpeed)) 0.0) false false))

(event Input|AxisEvents|InputAxisRoll
  (params (AxisValue :type Float%20%28single-precision%29))
  (Transformation|AddActorLocalRotation (Math|Rotator|MakeRotator 0.0 (* (Math|Float|Clamp(Float) AxisValue -1.0) (Utilities|Time|GetWorldDeltaSeconds) (Variables|Default|GetRotationSpeed)) 0.0) false false))

(fn ConstructionScript)

(fn RotatePropeller
  (params (self2 :type Scene%20Component%20Object%20Reference))
  (Transformation|AddLocalRotation self2 (Math|Rotator|MakeRotator (* (Utilities|Time|GetWorldDeltaSeconds) (Variables|속력|GetPropellerRotationSpeed)) 0.0 0.0) false false))