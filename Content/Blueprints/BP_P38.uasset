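; BP_P38 is an aircraft actor that flies in a straight line along world X while spinning its two propellers.
; Tick rolls both propellers by RotationSpeed, the right through the RotatePropeller function and the left through an inline copy of the same logic.
; It then offsets the actor by MoveSpeed, with all motion scaled by world delta seconds for frame-rate independence.
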(event EventBeginPlay)

(event Collision|EventActorBeginOverlap
  (params (OtherActor :type Actor%20Object%20Reference)))

(event EventTick
  (params (DeltaSeconds :type Float%20%28single-precision%29))
  ;[1 1 1] Rotate Right
  (CallFunction|RotatePropeller (Variables|Default|GetRightPropeller))
  ;[1 1 1] Rotate Left
  (Transformation|AddLocalRotation (Variables|Default|GetLeftPropeller) (Math|Rotator|MakeRotator (* (Utilities|Time|GetWorldDeltaSeconds) (Variables|속력|GetRotationSpeed)) 0.0 0.0) false false)
  ;[1 1 1] Move Plane
  (Transformation|AddActorWorldOffset (Math|Vector|MakeVector (* (Utilities|Time|GetWorldDeltaSeconds) (Variables|속력|GetMoveSpeed)) 0.0 0.0)))

(fn ConstructionScript)

(fn RotatePropeller
  (params (self2 :type Scene%20Component%20Object%20Reference))
  (Transformation|AddLocalRotation self2 (Math|Rotator|MakeRotator (* (Utilities|Time|GetWorldDeltaSeconds) (Variables|속력|GetRotationSpeed)) 0.0 0.0) false false))